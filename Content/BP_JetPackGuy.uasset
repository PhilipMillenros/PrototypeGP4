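; BP_JetPackGuy is a player-controlled physics jetpack character driven by a simulated Cube component.
; Space toggles thrusting, and A and D set an opposing roll torque value that resets to zero on release.
; While thrusting, Tick applies force along the cube's up vector plus torque around its forward vector, so steering only takes effect during thrust.
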(event EventBeginPlay)

(event Collision|EventActorBeginOverlap
  (params (OtherActor :type Actor%20Object%20Reference)))

(event EventTick
  (params (DeltaSeconds :type Float%20%28single-precision%29))
  (bind _cube (Variables|Default|GetCube))
  (if (Variables|Default|GetThrusting)
    (Physics|AddForce _cube (* (Math|Vector|GetUpVector _cube) (Variables|Default|GetThrustForce)) "None" false)
    (Class|PrimitiveComponent|AddTorqueinRadians (Variables|Default|GetCube) (* (Variables|Default|GetRotation) (Math|Vector|GetForwardVector (Variables|Default|GetCube))) "None" false)))

(event Input|KeyboardEvents|SpaceBar
  (params (Key :type Key%20Structure))
  (:Pressed
    (Variables|Default|SetThrusting true))
  (:Released
    (Variables|Default|SetThrusting false)))

(event Input|KeyboardEvents|A
  (params (Key :type Key%20Structure))
  (:Pressed
    (Variables|Default|SetRotation 4e+05))
  (:Released
    (Variables|Default|SetRotation 0.0)))

(event Input|KeyboardEvents|D
  (params (Key :type Key%20Structure))
  (:Pressed
    (Variables|Default|SetRotation -4e+05))
  (:Released
    (Variables|Default|SetRotation 0.0)))

(fn ConstructionScript)